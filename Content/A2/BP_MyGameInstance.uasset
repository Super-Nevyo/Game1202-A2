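; Game instance that persists the player's win count through a BP_MySaveData save in the default slot.
; On Init it loads the existing save and caches its win count, or creates and saves a new one if none exists.
; Triggered records a win behind the TempWin flag, incrementing, printing and immediately saving the count.
; The flag is never cleared here, so repeat triggers only print an already-won message.
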(event `self.ReceiveInit`
  (bind _returnvalue (`GameplayStatics.DoesSaveGameExist` (`self.DefaultSaveSlot`)))
  (if _returnvalue
    (bind _returnvalue_2 (`GameplayStatics.LoadGameFromSlot` (`self.DefaultSaveSlot`)))
    (bind _asbp_my_save_data (cast `/Game/A2/BP_MySaveData` _returnvalue_2))
    (bind _output_get (set `self.SaveGameData` _asbp_my_save_data))
    (set `self.tempWinNum` (`/Game/A2/BP_MySaveData.WinCount` _output_get))
    (else
      (bind _returnvalue_3 (`GameplayStatics.CreateSaveGameObject` "/Game/A2/BP_MySaveData.BP_MySaveData_C"))
      (bind _output_get_2 (set `self.SaveGameData` _returnvalue_3))
      (`GameplayStatics.SaveGameToSlot` _output_get_2 (`self.DefaultSaveSlot`)))))

(event `/Game/A2/InteractSystem/BPI_Triggerable.Triggered`
  (if (`self.tempWin`)
    (`KismetSystemLibrary.PrintString` "You won already")
    (else
      (set `self.tempWin` true)
      (bind _result (`/Engine/EditorBlueprintResources/StandardMacros.IncrementInt` (`self.tempWinNum`))
        (:`  `
          (`KismetSystemLibrary.PrintString` (`KismetStringLibrary.Conv_IntToString` _result))
          (set `/Game/A2/BP_MySaveData.WinCount` _result (`self.SaveGameData`))
          (`GameplayStatics.SaveGameToSlot` (`self.SaveGameData`) (`self.DefaultSaveSlot`)))))))
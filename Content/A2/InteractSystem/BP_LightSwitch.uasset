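; BP_LightSwitch is an interactable wall switch actor that turns a set of linked lights on and off.
; Its Interactwith event calls ToggleLight, which swaps the switch mesh between blue and pink materials and flips SwitchOn.
; ToggleLight then applies the new state as point light visibility on every actor in the LightSource array.
; GetInteractorPropmt returns "Turn Light Off" or "Turn Light On" to match the current state.
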(event `/Game/A2/InteractSystem/BPI_Interactable.InteractWith`
  (params (Interactor :type "Actor Object Reference"))
  (`self.ToggleLight`))

(fn `GetInteractorPropmt`
  (returns (PromptText :type Text))
  (if (`self.bSwitchOn`)
    (set `self.Prompt Text` "Turn Light Off")
    (else
      (bind _output_get (set `self.Prompt Text` "Turn Light On"))))
  (return _output_get))

(fn `ToggleLight`
  (if (`self.bSwitchOn`)
    (`PrimitiveComponent.SetMaterial` (`self.SwitchMesh`) 0 "/Game/A2/Materials/MI_Blue.MI_Blue")
    (else
      (`PrimitiveComponent.SetMaterial` (`self.SwitchMesh`) 0 "/Game/A2/Materials/MI_Pink.MI_Pink")))
  (bind _output_get (set `self.bSwitchOn` (not (`self.bSwitchOn`))))
  (for _array_element (`self.LightSource`)
    (`SceneComponent.SetVisibility` (`/Game/A2/BP_LightSource.PointLight` _array_element) _output_get false)))

(fn `UserConstructionScript`)
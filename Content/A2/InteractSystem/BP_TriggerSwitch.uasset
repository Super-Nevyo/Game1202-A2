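; BP_TriggerSwitch is an interactable wall switch that triggers a list of linked objects and can act as a win button.
; On interact it plays a sound, sends TriggeredMessage to each entry in Triggerables and spawns a Niagara burst on the switch.
; When flagged as the win button, it also sends TriggeredMessage to the Game Instance.
; It returns its PromptText as the interaction prompt.
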(event `/Game/A2/InteractSystem/BPI_Interactable.InteractWith`
  (params (Interactor :type "Actor Object Reference"))
  (`GameplayStatics.PlaySound2D` "/Engine/VREditor/Sounds/UI/Camera_Shutter.Camera_Shutter" 1.0 1.0 0.0 null null)
  (for _array_element (`self.Triggerables`)
    (message `/Game/A2/InteractSystem/BPI_Triggerable.Triggered` _array_element))
  (`NiagaraFunctionLibrary.SpawnSystemAttached` "/Game/A2/VFX/NS_SwitchBurst.NS_SwitchBurst" (`self.WallSwitch`) "None" (0.0 1.0 0.0) (struct) "KeepRelativeOffset" true)
  (if (`self.IsThisWinButton`)
    (message `/Game/A2/InteractSystem/BPI_Triggerable.Triggered` (`GameplayStatics.GetGameInstance`))))

(fn `GetInteractorPropmt`
  (returns (PromptText :type Text))
  (return (`self.Prompt Text`)))

(fn `UserConstructionScript`)
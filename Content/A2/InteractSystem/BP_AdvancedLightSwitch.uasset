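; BP_AdvancedLightSwitch is an interactable light switch that toggles its light and plays a level sequence when used.
; On BeginPlay it caches the LevelSequenceActor returned by GetActorOfClass, so the sequence is found by class search rather than by a specific reference.
; The Interactwith event calls ToggleLight, then plays that sequence through its SequencePlayer, with no validity check.
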(event `self.ReceiveBeginPlay`
  (`parent.ReceiveBeginPlay`)
  (bind _returnvalue (`GameplayStatics.GetActorOfClass` "/Script/LevelSequence.LevelSequenceActor"))
  (set `self.LightSequence` _returnvalue))

(event `/Game/A2/InteractSystem/BPI_Interactable.InteractWith`
  (params (Interactor :type "Actor Object Reference"))
  (`self.ToggleLight`)
  (`MovieSceneSequencePlayer.Play` (`LevelSequenceActor.SequencePlayer` (`self.LightSequence`))))

(fn `UserConstructionScript`
  (`parent.UserConstructionScript`))
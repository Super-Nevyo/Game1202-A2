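; BP_MovingWall is a wall actor that slides between its starting transform and a configurable destination when triggered.
; BeginPlay caches the wall's world transform, and the WallMovement timeline lerps from it to DestinationLocation, whose location is offset from the root while rotation and scale apply as-is.
; Triggered toggles between playing and reversing the timeline based on IsOn, while UnTriggered always sets IsOn and reverses it.
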(event `self.ReceiveBeginPlay`
  (set `self.OriginLocation` (`SceneComponent.K2_GetComponentToWorld` (`self.MovingWall`))))

(event `/Game/A2/InteractSystem/BPI_Triggerable.Triggered`
  (bind (_destinationlocation_location _destinationlocation_rotation _destinationlocation_scale) (`KismetMathLibrary.BreakTransform` (`self.DestinationLocation`)))
  (bind _returnvalue_location (`KismetMathLibrary.BreakTransform` (`SceneComponent.K2_GetComponentToWorld` (`self.DefaultSceneRoot`))))
  (if (`self.IsOn`)
    (set `self.IsOn` false)
    (bind (_direction _newtrack_0) (`Timeline|WallMovement` :!label _label)
      (:`Update`
        (`SceneComponent.K2_SetWorldTransform` (`self.MovingWall`) (`KismetMathLibrary.TLerp` (`self.OriginLocation`) (`KismetMathLibrary.MakeTransform` (+ _destinationlocation_location _returnvalue_location) _destinationlocation_rotation _destinationlocation_scale) _newtrack_0) false false)))
    (else
      (set `self.IsOn` true :!label _label_2)
      (goto _label :!via `Reverse`))))

(event `/Game/A2/InteractSystem/BPI_Triggerable.UnTriggered`
  (goto _label_2))

(fn `UserConstructionScript`)